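; Player Blueprint for a physics-driven ball, handling savepoint respawns, death counting and audio.
; BeginPlay stores the ball's location as the savepoint; Respawn teleports there, resets rotation and velocities, and copies the incremented death count to GI_Point.
; Sound events play one-shot cues, and BGMChange swaps the current music.
; Hotkeys reload MudFlat, open EndLevel, warp to CheatPoint or add deaths, while Tick prints ball height for debugging.
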(event `self.ReceiveBeginPlay`
  (cast `Orange` (`GameplayStatics.GetPlayerPawn` 0))
  (set `self.Savepoint` (`SceneComponent.K2_GetComponentLocation` (`self.Ball`))))

(event `self.ReceiveTick`
  (params (DeltaSeconds :type "Float (single-precision)"))
  (bind (_returnvalue_x _returnvalue_y _returnvalue_z) (`KismetMathLibrary.BreakVector` (`SceneComponent.K2_GetComponentLocation` (`self.Ball`))))
  (`KismetSystemLibrary.PrintString` (`KismetStringLibrary.Conv_DoubleToString` _returnvalue_z) false false (struct :`G` 0.66 :`B` 1.0 :`A` 1.0) DeltaSeconds)
  (if (< _returnvalue_z 200.0)
    _))

(event `Key|R`
  (params (Key :type "Key Structure"))
  (:`Pressed`
    (`GameplayStatics.OpenLevelBySoftObjectPtr` "/Game/Map/MudFlat.MudFlat")))

(event `Key|Zero`
  (params (Key :type "Key Structure"))
  (:`Pressed`
    (`self.K2_TeleportTo` (`self.CheatPoint`))
    (`SceneComponent.K2_SetRelativeRotation` (`self.Ball`) (struct :`Yaw` 90.0) false false)
    (`PrimitiveComponent.SetPhysicsLinearVelocity` (`self.Ball`) (0.0 0.0 0.0) false "None")
    (`PrimitiveComponent.SetPhysicsAngularVelocityInDegrees` (`self.Ball`) (0.0 0.0 0.0) false "None")))

(event `self.SoundQueue`
  (`GameplayStatics.PlaySound2D` "/Game/Sound/jump.jump" 1.0 1.0 0.0 null null))

(event `self.DeadSoundQueue`
  (`GameplayStatics.PlaySound2D` "/Game/Sound/dropping_Ocean.dropping_Ocean" 1.0 1.0 0.0 null null))

(event `Key|Equals`
  (params (Key :type "Key Structure"))
  (:`Pressed`
    (bind _output_get (set `self.DeadCount` (+ (`self.DeadCount`) 1)))
    (bind _asgi_point (cast `/Game/Gamemode/GI_Point` (`GameplayStatics.GetGameInstance`)))
    (set `/Game/Gamemode/GI_Point.DeadCount` _output_get _asgi_point)))

(event `self.SaveSoundQueue`
  (`GameplayStatics.PlaySound2D` "/Game/Sound/save_point.save_point" 1.0 1.0 0.0 null null))

(event `self.HeadingSoundQueue`
  (`GameplayStatics.PlaySound2D` "/Game/Sound/dropping.dropping" 1.0 1.0 0.0 null null))

(event `Key|Hyphen`
  (params (Key :type "Key Structure"))
  (:`Pressed`
    (`GameplayStatics.OpenLevelBySoftObjectPtr` "/Game/Map/EndLevel.EndLevel")))

(fn `BGM Change`
  (params (`New Sound` :type "SoundBase Object Reference"))
  (bind _currentbgm (`self.CurrentBGM`))
  (`/Engine/EditorBlueprintResources/StandardMacros.IsValid` _currentbgm
    (:`Is Valid`
      (`AudioComponent.Stop` _currentbgm))
    (:`Is Not Valid`
      _))
  (bind _returnvalue (`GameplayStatics.SpawnSound2D` `New Sound` 1.0 1.0 0.0 null))
  (set `self.CurrentBGM` _returnvalue))

(fn `Respawn`
  (`self.DeadSoundQueue`)
  (`self.K2_TeleportTo` (`self.Savepoint`))
  (`SceneComponent.K2_SetRelativeRotation` (`self.Ball`) (struct :`Yaw` 90.0) false false)
  (`PrimitiveComponent.SetPhysicsLinearVelocity` (`self.Ball`) (0.0 0.0 0.0) false "None")
  (`PrimitiveComponent.SetPhysicsAngularVelocityInDegrees` (`self.Ball`) (0.0 0.0 0.0) false "None")
  (bind _output_get (set `self.DeadCount` (+ (`self.DeadCount`) 1)))
  (bind _asgi_point (cast `/Game/Gamemode/GI_Point` (`GameplayStatics.GetGameInstance`)))
  (set `/Game/Gamemode/GI_Point.DeadCount` _output_get _asgi_point))

(fn `UserConstructionScript`)