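; SuitCase is a checkpoint object that sets the player's respawn savepoint on touch.
; The construction script places the spawn point slightly above its Box component.
; When a Player overlaps the Box, it receives that point as its Savepoint, and the save sound plays only on the first such overlap.
; Other overlapping actors only trigger a debug print.
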(event `self.Box.OnComponentBeginOverlap`
  (params (OverlappedComponent :type "PrimitiveComponent Object Reference") (OtherActor :type "Actor Object Reference") (OtherComp :type "PrimitiveComponent Object Reference") (OtherBodyIndex :type Integer) (bFromSweep :type Boolean) (SweepResult :type "HitResult Structure (by ref)"))
  (bind _asplayer (cast `/Game/Orange/Blueprints/Player` OtherActor)
    (:`then`
      (if (not (`self.bPlayedSaveSound`))
        (`Orange.SaveSoundQueue` _asplayer)
        (set `self.bPlayedSaveSound` true))
      (set `/Game/Orange/Blueprints/Player.Savepoint` (`self.Spawnpoint`) _asplayer))
    (:`CastFailed`
      (`KismetSystemLibrary.PrintString` "Hello"))))

(fn `UserConstructionScript`
  (set `self.Spawnpoint` (+ (`SceneComponent.K2_GetComponentLocation` (`self.Box`)) (0.0 0.0 100.0))))