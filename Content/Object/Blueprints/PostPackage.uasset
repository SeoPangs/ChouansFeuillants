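; PostPackage is an actor with a Box trigger that lowers its Arrow component after an Orange has spent enough time inside.
; Box overlap events toggle OnSphere, and Tick adds to StepTimer while it is set.
; Past three seconds, the Arrow moves steadily down without sweep for as long as the Orange stays inside.
; StepTimer never resets, so time accumulates across visits, and debug prints show timer and overlap state.
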(event `self.ReceiveTick`
  (params (DeltaSeconds :type "Float (single-precision)"))
  (if (`self.bOnSphere`)
    (bind _output_get (set `self.StepTimer` (+ DeltaSeconds (`self.StepTimer`))))
    (`KismetSystemLibrary.PrintString` (`KismetStringLibrary.Conv_DoubleToString` _output_get) true true (struct :`G` 0.554167 :`B` 0.041464 :`A` 1.0) DeltaSeconds)
    (if (> (`self.StepTimer`) 3.0)
      (`SceneComponent.K2_SetRelativeLocation` (`self.Arrow`) (+ (`SceneComponent.RelativeLocation` (`self.Arrow`)) (`KismetMathLibrary.MakeVector` 0.0 0.0 (* -100 DeltaSeconds))) false false))))

(event `self.Box.OnComponentBeginOverlap`
  (params (OverlappedComponent :type "PrimitiveComponent Object Reference") (OtherActor :type "Actor Object Reference") (OtherComp :type "PrimitiveComponent Object Reference") (OtherBodyIndex :type Integer) (bFromSweep :type Boolean) (SweepResult :type "HitResult Structure (by ref)"))
  (cast `Orange` OtherActor)
  (bind _output_get (set `self.bOnSphere` true))
  (`KismetSystemLibrary.PrintString` (`KismetStringLibrary.Conv_BoolToString` _output_get)))

(event `self.Box.OnComponentEndOverlap`
  (params (OverlappedComponent :type "PrimitiveComponent Object Reference") (OtherActor :type "Actor Object Reference") (OtherComp :type "PrimitiveComponent Object Reference") (OtherBodyIndex :type Integer))
  (cast `Orange` OtherActor)
  (bind _output_get (set `self.bOnSphere` false))
  (`KismetSystemLibrary.PrintString` (`KismetStringLibrary.Conv_BoolToString` _output_get)))

(fn `UserConstructionScript`)