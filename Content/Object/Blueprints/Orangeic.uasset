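; Orangeic is a Blueprint with a physics Ball component that handles respawning at a savepoint and switching background music.
; Respawn triggers the death sound, teleports the actor to the savepoint, resets the Ball's rotation and linear and angular velocities, then increments the death count.
; BGM Change stops any valid current track, spawns the new sound in 2D and stores it as the current music.
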(fn `BGM Change`
  (params (`New Sound` :type "SoundBase Object Reference"))
  (bind _currentbgm (`self.CurrentBGM`))
  (`/Engine/EditorBlueprintResources/StandardMacros.IsValid` _currentbgm
    (:`Is Valid`
      (`AudioComponent.Stop` _currentbgm))
    (:`Is Not Valid`
      _))
  (bind _returnvalue (`GameplayStatics.SpawnSound2D` `New Sound` 1.0 1.0 0.0 null))
  (set `self.CurrentBGM` _returnvalue))

(fn `Respawn`
  (`self.DeadSoundQueue`)
  (`self.K2_TeleportTo` (`self.Savepoint`))
  (`SceneComponent.K2_SetRelativeRotation` (`self.Ball`) (struct :`Yaw` 90.0) false false)
  (`PrimitiveComponent.SetPhysicsLinearVelocity` (`self.Ball`) (0.0 0.0 0.0) false "None")
  (`PrimitiveComponent.SetPhysicsAngularVelocityInDegrees` (`self.Ball`) (0.0 0.0 0.0) false "None")
  (set `self.DeadCount` (+ (`self.DeadCount`) 1)))

(fn `UserConstructionScript`)